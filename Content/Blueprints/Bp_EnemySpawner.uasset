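; Spawner Blueprint that populates the level with AI enemies when play begins.
; It finds every BP_EnemySpawnPoint and spawns one BP_AiMoveTo at each transform, ignoring collisions.
; Each spawned AI's AIName text is set to a random AINames entry, indexed by a truncated random float, so names can repeat.
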(event `self.ReceiveBeginPlay`
  (bind _ainames (`self.AINames`))
  (bind _outactors (`GameplayStatics.GetAllActorsOfClass` "/Game/Blueprints/BP_EnemySpawnPoint.BP_EnemySpawnPoint_C"))
  (for _array_element _outactors
    (bind _returnvalue (`|SpawnActorFromClass` "/Game/AI_Blueprints/BP_AiMoveTo.BP_AiMoveTo_C" (`self.GetTransform` _array_element) "AlwaysSpawn" "MultiplyWithRoot" null null))
    (`TextRenderComponent.K2_SetText` (`/Game/AI_Blueprints/BP_AiMoveTo.AIName` _returnvalue) (`|GetArrayItem` _ainames (`KismetMathLibrary.FTrunc` (`KismetMathLibrary.RandomFloatInRange` 0.0 (`KismetMathLibrary.Conv_IntToDouble` (`KismetArrayLibrary.Array_Length` _ainames))))))))

(fn `UserConstructionScript`)