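; Key-gated door actor that lowers its Cube when a character holding at least one key enters the Box trigger.
; On overlap, it reads Keys from BP_ThirdPersonCharacter and plays the OpenDoor timeline, which lerps the Cube's relative Z, or prints "key needed".
; Keys are only checked, never consumed, and the timeline reverses when player 0's character leaves the trigger.
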(event `self.Box.OnComponentBeginOverlap`
  (params (OverlappedComponent :type "PrimitiveComponent Object Reference") (OtherActor :type "Actor Object Reference") (OtherComp :type "PrimitiveComponent Object Reference") (OtherBodyIndex :type Integer) (bFromSweep :type Boolean) (SweepResult :type "HitResult Structure (by ref)"))
  (if (>= (`/Game/ThirdPerson/Blueprints/BP_ThirdPersonCharacter.Keys` (cast `/Game/ThirdPerson/Blueprints/BP_ThirdPersonCharacter` OtherActor :!pure true)) 1)
    (bind (_direction _newtrack_0) (`Timeline|OpenDoor` :!label _label)
      (:`Update`
        (`SceneComponent.K2_SetRelativeLocation` (`self.Cube`) (`KismetMathLibrary.MakeVector` 0.0 0.0 (`KismetMathLibrary.Lerp` 160.0 -160.0 _newtrack_0)) false false)))
    (else
      (`KismetSystemLibrary.PrintString` "key needed"))))

(event `self.Box.OnComponentEndOverlap`
  (params (OverlappedComponent :type "PrimitiveComponent Object Reference") (OtherActor :type "Actor Object Reference") (OtherComp :type "PrimitiveComponent Object Reference") (OtherBodyIndex :type Integer))
  (if (== OtherActor (`GameplayStatics.GetPlayerCharacter` 0))
    (goto _label :!via `Reverse`)))

(fn `UserConstructionScript`)